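; BP_Point_Light is a configurable point light actor for placing lights in levels.
; Its construction script copies exposed variables onto the PointLight component, covering intensity, attenuation, source shape, lighting channels, shadow casting and inverse-squared falloff.
; The event graph holds only disabled placeholder events, so the actor has no runtime logic.
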(fn `UserConstructionScript`
  (`LightComponent.SetIntensity` (`self.PointLight`) (`self.strength`))
  (`LocalLightComponent.SetAttenuationRadius` (`self.PointLight`) (`self.attenuationRad`))
  (`LightComponent.SetLightingChannels` (`self.PointLight`) (`self.channel0`) (`self.channel1`) (`self.channel2`))
  (`PointLightComponent.SetSourceRadius` (`self.PointLight`) (`self.sourceRadius`))
  (`PointLightComponent.SetSoftSourceRadius` (`self.PointLight`) (`self.softSourceRadius`))
  (`PointLightComponent.SetSourceLength` (`self.PointLight`) (`self.sourceLength`))
  (`LightComponentBase.SetCastShadows` (`self.PointLight`) (`self.castShadow`))
  (`PointLightComponent.SetUseInverseSquaredFalloff` (`self.PointLight`) (`self.userInverseFallOff`)))