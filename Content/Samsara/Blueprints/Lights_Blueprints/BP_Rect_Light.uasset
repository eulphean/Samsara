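; BP_Rect_Light is a rect light actor Blueprint that applies its settings from its own variables.
; The construction script pushes source size, attenuation radius, intensity, lighting channels and shadow casting onto the RectLight component.
; The event graph holds only disabled placeholder events, so the Blueprint adds no runtime logic.
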(fn `UserConstructionScript`
  (`RectLightComponent.SetSourceWidth` (`self.RectLight`) (`self.sourceWidth`))
  (`RectLightComponent.SetSourceHeight` (`self.RectLight`) (`self.sourceHeight`))
  (`LocalLightComponent.SetAttenuationRadius` (`self.RectLight`) (`self.attenuationRadius`))
  (`LightComponent.SetIntensity` (`self.RectLight`) (`self.strength`))
  (`LightComponent.SetLightingChannels` (`self.RectLight`) (`self.channel0`) (`self.channel1`) (`self.channel2`))
  (`LightComponentBase.SetCastShadows` (`self.RectLight`) (`self.castShadow`)))