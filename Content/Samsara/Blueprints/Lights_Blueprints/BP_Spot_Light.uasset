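; BP_Spot_Light is a configurable spot light actor for placing lighting in a level.
; Its construction script copies exposed variables onto the SpotLight component, setting intensity, inner and outer cone angles, lighting channels and attenuation radius.
; The event graph holds only disabled placeholder events, so the Blueprint adds no runtime logic.
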(fn `UserConstructionScript`
  (`LightComponent.SetIntensity` (`self.SpotLight`) (`self.strength`))
  (`SpotLightComponent.SetOuterConeAngle` (`self.SpotLight`) (`self.outerConeAngle`))
  (`SpotLightComponent.SetInnerConeAngle` (`self.SpotLight`) (`self.innerConeAngle`))
  (`LightComponent.SetLightingChannels` (`self.SpotLight`) (`self.channel0`) (`self.channel1`) (`self.channel2`))
  (`LocalLightComponent.SetAttenuationRadius` (`self.SpotLight`) (`self.attentuationRad`)))