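; Archived architectural layout manager that places instanced pillars, frames, ceilings and floors along a spline in the Construction Script.
; CreateInstanceMesh selects spacing by mesh type, then adds world-space instances using spline location and rotation.
; Pillars and frames divide the spline length by a set count, plus an offset.
; Ceilings and floors take spacing from mesh X bounds but never set an instance count, and their type labels are swapped.
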(fn `createInstanceMesh`
  (params (splineLength :type "Float (double-precision)") (instancedMesh :type "InstancedStaticMeshComponent Object Reference") (meshType :type String) (offset :type "Float (double-precision)") (scale :type "Vector Structure") (numMeshes :type Integer))
  (locals (spacing :type "Float (double-precision)") (numInstances :type Integer))
  (bind _returnvalue (- (`local.numMeshes`) 1))
  (bind (_min _max) (break `Box` (`StaticMesh.GetBoundingBox` (`StaticMeshComponent.StaticMesh` (`local.instancedMesh`)))))
  (switch `string` (`local.meshType`)
    (:`frame`
      (set `local.spacing` (+ (/ (`local.splineLength`) _returnvalue) (`local.offset`)) :!label _label)
      (set `local.numInstances` _returnvalue))
    (:`pillar`
      (goto _label))
    (:`ceiling`
      (set `local.spacing` (.x (- _max _min)) :!label _label_2))
    (:`floor`
      (goto _label_2)))
  (for _index (range (+ (`local.numInstances`) 1))
    (`InstancedStaticMeshComponent.AddInstance` (`local.instancedMesh`) (`KismetMathLibrary.MakeTransform` (.location (`SplineComponent.GetTransformAtDistanceAlongSpline` (`self.splineController`) (* _index (`local.spacing`)) "World" true)) (.rotation (`SplineComponent.GetTransformAtDistanceAlongSpline` (`self.splineController`) (* _index (`local.spacing`)) "World" true)) (`local.scale`)) true)))

(fn `UserConstructionScript`
  (locals (splineLength :type "Float (single-precision)" :default 0.0) (floorSpacing :type "Float (double-precision)"))
  (`|ExecutionSequence`
    (:`then_0`
      (set `local.splineLength` (`SplineComponent.GetSplineLength` (`self.splineController`))))
    (:`then_1`
      (`self.createInstanceMesh` (`local.splineLength`) (`self.PillarInstancedMesh`) "pillar" (`self.pOffset`) (1.0 1.0 1.0) (`self.numPillars`))
      (`self.createInstanceMesh` (`local.splineLength`) (`self.CeilingInstancedMesh`) "floor" 0.0 (1.0 1.0 1.0))
      (`self.createInstanceMesh` (`local.splineLength`) (`self.FloorInstancedMesh`) "ceiling" 0.0 (1.0 1.0 1.0))
      (`self.createInstanceMesh` (`local.splineLength`) (`self.FrameInstancedMesh`) "frame" (`self.fOffset`) (`self.fScale`) (`self.numFrames`)))))