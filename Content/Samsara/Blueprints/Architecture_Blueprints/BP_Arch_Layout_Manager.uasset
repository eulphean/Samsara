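; Architecture layout manager that builds a spline-driven structure of pillars, frames, ceiling, floor and side pillars from instanced meshes.
; The construction script passes each part's instanced mesh, static mesh and scale, plus a shared spline controller, to that part's handler via SetupMeshInstance.
; Pillars, frames and side pillars also take a count and offset.
; All work happens at construction; the event graph is empty.
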(fn `UserConstructionScript`
  (locals (splineLength :type "Float (single-precision)" :default 0.0))
  (`/Game/Samsara/Blueprints/Architecture_Blueprints/Mesh_Handlers/BP_MeshHandler.setupMeshInstance` (`self.BP_PillarHandler`) (`self.PillarInstancedMesh`) (`self.splineController`) (`self.pScale`) (`self.numPillars`) (`self.pOffset`) (`self.pillarMesh`) (`self.Scene`))
  (`/Game/Samsara/Blueprints/Architecture_Blueprints/Mesh_Handlers/BP_MeshHandler.setupMeshInstance` (`self.BP_FrameHandler`) (`self.FrameInstancedMesh`) (`self.splineController`) (`self.fScale`) (`self.numFrames`) (`self.fOffset`) (`self.frameMesh`) (`self.Scene`))
  (`/Game/Samsara/Blueprints/Architecture_Blueprints/Mesh_Handlers/BP_MeshHandler.setupMeshInstance` (`self.BP_CeilingHandler`) (`self.CeilingInstancedMesh`) (`self.splineController`) (`self.cScale`) 0 0.0 (`self.ceilingMesh`) (`self.Scene`))
  (`/Game/Samsara/Blueprints/Architecture_Blueprints/Mesh_Handlers/BP_MeshHandler.setupMeshInstance` (`self.BP_FloorHandler`) (`self.FloorInstancedMesh`) (`self.splineController`) (`self.floorScale`) 0 0.0 (`self.floorMesh`) (`self.Scene`))
  (`/Game/Samsara/Blueprints/Architecture_Blueprints/Mesh_Handlers/BP_MeshHandler.setupMeshInstance` (`self.BP_Child_SidePillarHandler`) (`self.SidePillarInstancedMesh`) (`self.splineController`) (`self.spScale`) (`self.numSidePillars`) (`self.spOffset`) (`self.spMesh`) null))