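; Child mesh handler Blueprint that places frame mesh instances along a spline, intended to sit midway between pillars.
; It overrides SetupMeshInstance, calls the parent, then divides spline length by mesh count to get the spacing.
; Each world-space instance takes its spline transform, shifted half a spacing along X rather than along the spline.
; Each instance's index is written as per-instance custom data for material variation.
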(fn `setupMeshInstance`
  (params (instancedMesh :type "InstancedStaticMeshComponent Object Reference") (splineController :type "SplineComponent Object Reference") (scale :type "Vector Structure") (numMeshes :type Integer) (offset :type "Float (double-precision)") (staticMesh :type "StaticMesh Object Reference") (scene :type "SceneComponent Object Reference"))
  (locals (splineLength :type "Float (double-precision)") (spacing :type "Float (double-precision)") (lastIdx :type Integer) (curLoopIdx :type Integer))
  (bind _nummeshes (`self.numMeshes`))
  (bind _instancedmesh (`local.instancedMesh`))
  (bind _curloopidx (`local.curLoopIdx`))
  (`parent.setupMeshInstance` instancedMesh splineController scale numMeshes offset staticMesh scene)
  ; Comment
  (bind _output_get (set `local.splineLength` (`SplineComponent.GetSplineLength` (`local.splineController`))))
  (set `local.spacing` (/ _output_get _nummeshes))
  ; Last Index (-1 because it starts at 0)
  (bind _output_get_2 (set `local.lastIdx` (- _nummeshes 1)))
  (for _index (range (+ _output_get_2 1))
    (bind _output_get_3 (set `local.curLoopIdx` _index))
    (bind _transform (`self.getTransformAlongSpline` (`local.splineController`) (`local.scene`) (`local.spacing`) _output_get_3))
    (`InstancedStaticMeshComponent.AddInstance` (`local.instancedMesh`) (`KismetMathLibrary.MakeTransform` (`KismetMathLibrary.MakeVector` (+ (.x (.location _transform)) (/ (`local.spacing`) 2.0)) (.y (.location _transform)) (.z (.location _transform))) (.rotation _transform) (.scale _transform)) true)
    ; Add custom data value per instance (Access them in material to change material per instance)
    (`InstancedStaticMeshComponent.SetNumCustomDataFloats` _instancedmesh 1)
    (`InstancedStaticMeshComponent.SetCustomDataValue` _instancedmesh _curloopidx 0 (`KismetMathLibrary.Conv_IntToDouble` _curloopidx) true)))