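; BP_MeshHandler is a helper that distributes instanced static meshes along a spline.
; A setup function stores mesh, scale, count and offset, then instances are placed either repeatedly by mesh X size or by count with offset-adjusted spacing.
; Transforms take only X from the spline, with Y and Z from a scene component and zero rotation.
; Count-based placement also writes each instance's index to custom data for per-instance material variation.
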(fn `createInstancesByNum`
  (params (instancedMesh :type "InstancedStaticMeshComponent Object Reference") (splineController :type "SplineComponent Object Reference") (scene :type "SceneComponent Object Reference"))
  (locals (spacing :type "Float (double-precision)") (lastIndex :type Integer) (splineLength :type "Float (single-precision)" :default 0.0) (curLoopIndex :type Integer))
  (bind _curloopindex (`local.curLoopIndex`))
  (bind _returnvalue (- (`self.localNumMeshes`) 1))
  ; Capture current spline length
  (bind _output_get (set `local.splineLength` (`SplineComponent.GetSplineLength` (`local.splineController`))))
  ; Take localOffset into account for spacing
  (set `local.spacing` (+ (/ _output_get _returnvalue) (`self.localOffset`)))
  ; Update last index
  (bind _output_get_2 (set `local.lastIndex` _returnvalue))
  ; For each num in numInstances, calculate point along the spline (with calculated spacing)
  (for _index (range (+ _output_get_2 1))
    (bind _output_get_3 (set `local.curLoopIndex` _index))
    (bind _transform (`self.getTransformAlongSpline` (`local.splineController`) (`local.scene`) (`local.spacing`) _output_get_3))
    ; Add Instance
    (`InstancedStaticMeshComponent.AddInstance` (`local.instancedMesh`) _transform true)
    ; Add custom data value per instance (Access them in material to change material per instance)
    (`InstancedStaticMeshComponent.SetNumCustomDataFloats` (`local.instancedMesh`) 1)
    (`InstancedStaticMeshComponent.SetCustomDataValue` (`local.instancedMesh`) _curloopindex 0 (`KismetMathLibrary.Conv_IntToDouble` _curloopindex) true)))

(fn `createRepeatedInstances`
  (params (instancedMesh :type "InstancedStaticMeshComponent Object Reference") (splineController :type "SplineComponent Object Reference") (scene :type "SceneComponent Object Reference"))
  (locals (splineLength :type "Float (double-precision)") (spacing :type "Float (double-precision)") (lastIndex :type Integer))
  (bind _spacing (`local.spacing`))
  (bind (_min _max) (break `Box` (`StaticMesh.GetBoundingBox` (`StaticMeshComponent.StaticMesh` (`local.instancedMesh`)))))
  (set `local.spacing` (.x (- _max _min)))
  ; Capture current length the spline
  (set `local.splineLength` (`SplineComponent.GetSplineLength` (`local.splineController`)))
  ; Calculate number of instances required
  (`KismetSystemLibrary.PrintString` (`KismetStringLibrary.Conv_DoubleToString` _spacing))
  (bind _output_get (set `local.lastIndex` (`KismetMathLibrary.FFloor` (/ (`local.splineLength`) _spacing))))
  ; For each instance, calculate the point on spline where it should lie
  (for _index (range (+ _output_get 1))
    (bind _transform (`self.getTransformAlongSpline` (`local.splineController`) (`local.scene`) (`local.spacing`) _index))
    ; Add Instance
    (`InstancedStaticMeshComponent.AddInstance` (`local.instancedMesh`) _transform true)))

(fn `getTransformAlongSpline`
  (params (splineController :type "SplineComponent Object Reference") (scene :type "SceneComponent Object Reference") (spacing :type "Float (double-precision)") (index :type Integer))
  (returns (transform :type "Transform Structure"))
  ; Given a current index, create a transform along the spline.
  (return (`KismetMathLibrary.MakeTransform` (`KismetMathLibrary.MakeVector` (.x (.location (`SplineComponent.GetTransformAtDistanceAlongSpline` (`local.splineController`) (* (`local.index`) (`local.spacing`)) "World" true))) (.y (`self.K2_GetComponentLocation` (`local.scene`))) (.z (`self.K2_GetComponentLocation` (`local.scene`)))) (struct) (`self.localScale`))))

(fn `setupMeshInstance`
  (params (instancedMesh :type "InstancedStaticMeshComponent Object Reference") (splineController :type "SplineComponent Object Reference") (scale :type "Vector Structure") (numMeshes :type Integer) (offset :type "Float (double-precision)") (staticMesh :type "StaticMesh Object Reference") (scene :type "SceneComponent Object Reference"))
  ; Setup the static mesh instance to be used when distributing the meshes
  (set `self.localScale` scale)
  (set `self.localNumMeshes` numMeshes)
  (bind _output_get (set `self.localStaticMesh` staticMesh))
  (set `self.localOffset` offset)
  (`StaticMeshComponent.SetStaticMesh` (`local.instancedMesh`) _output_get))