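; Side pillar mesh handler, a child Blueprint that sets up instanced pillar meshes from a spline controller for Samsara's architecture Blueprints.
; Its setup override runs the parent setup, then creates the instances by count.
; It then turns the second instance (index 1) by combining its rotation with a 180-degree pitch, keeping its local location and scale.
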(fn `setupMeshInstance`
  (params (instancedMesh :type "InstancedStaticMeshComponent Object Reference") (splineController :type "SplineComponent Object Reference") (scale :type "Vector Structure") (numMeshes :type Integer) (offset :type "Float (double-precision)") (staticMesh :type "StaticMesh Object Reference") (scene :type "SceneComponent Object Reference"))
  (bind _instancedmesh (`local.instancedMesh`))
  (`parent.setupMeshInstance` instancedMesh splineController scale numMeshes offset staticMesh scene)
  (`self.createInstancesByNum` (`local.instancedMesh`) (`local.splineController`))
  (`InstancedStaticMeshComponent.UpdateInstanceTransform` _instancedmesh 1 (`KismetMathLibrary.MakeTransform` (.location (`InstancedStaticMeshComponent.GetInstanceTransform` _instancedmesh 1 false)) (`KismetMathLibrary.ComposeRotators` (.rotation (`InstancedStaticMeshComponent.GetInstanceTransform` _instancedmesh 1 false)) (`KismetMathLibrary.MakeRotator` 0.0 180.0)) (.scale (`InstancedStaticMeshComponent.GetInstanceTransform` _instancedmesh 1 false))) false false false))