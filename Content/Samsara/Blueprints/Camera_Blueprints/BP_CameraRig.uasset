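; Camera rig actor that batch-renders a master sequence from up to ten cine cameras through Movie Render Queue.
; The construction script shapes a spline, positions and configures cameras from CameraConfig, and activates a preview camera.
; On BeginPlay it renders the chosen camera range sequentially, each finished job triggering the next.
; Each job activates one camera, enables only its mapped Sequencer media tracks and sets per-camera output names.
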(event `self.ReceiveBeginPlay`
  (bind _returnvalue (subsystem `MoviePipelineQueueEngineSubsystem`))
  (set `self.mrq` _returnvalue)
  ; Empty any existing jobs
  (`MoviePipelineQueue.DeleteAllJobs` (`MoviePipelineQueueEngineSubsystem.GetQueue` _returnvalue))
  ; Update the current camera. We cannot choose CineCameraComponents here since those are components. We need to choose actors. Since they are part of the BP_CameraRig actor, we just set the active camera on that and set the NewViewTarget to self. And it shows the correct camera because that's what we have chosen as the activeCamera in the beginning.
  (`PlayerController.SetViewTargetWithBlend` (`GameplayStatics.GetPlayerController` 0) self 0.0 "VTBlend_Linear" 0.0 false)
  (`self.CreateJobs`))

(event `CreateJobs`
  (set `self.curCamIdx` (`self.startCamIdx`))
  ; Should we setup a new job?
  (if (<= (`self.curCamIdx`) (`self.endCamIdx`)) :!label _label
    ; Set the right camera
    (`self.setActiveCamera` (`self.curCamIdx`))
    ; Enable / Disable media tracks for the current camera.
    (`self.enableMediaTracks` (`self.curCamIdx`))
    ; Setup the job and kickoff a render.
    (bind _returnvalue (`MoviePipelineQueueEngineSubsystem.AllocateJob` (`self.mrq`) (`self.masterSequence`)))
    (bind _output_get (set `self.curRenderJob` _returnvalue))
    (`self.updateOutputNames` _output_get (`self.curCamIdx`))
    (`MoviePipelineExecutorJob.SetConfiguration` (`self.curRenderJob`) (`self.renderConfig`))
    (`self.renderJob`)
    (else
      (`self.endRenderQueue`))))

(event `endRenderQueue`
  (bind _mrq (`self.mrq`))
  (bind _returnvalue (`MoviePipelineQueueEngineSubsystem.GetActiveExecutor` _mrq))
  ; Cleaning end the rendering process by deleting any pending jobs with mrq.
  (if (`KismetSystemLibrary.IsValid` _mrq)
    (if (`KismetSystemLibrary.IsValid` _returnvalue)
      (`MoviePipelineExecutorBase.CancelAllJobs` _returnvalue)
      (`KismetSystemLibrary.PrintString` "Render Cancelled")
      (else
        (`KismetSystemLibrary.PrintString` "No Active Jobs")))))

(event `renderJob`
  ; Render the current job
  (`MoviePipelineQueueEngineSubsystem.RenderJob` (`self.mrq`) (`self.curRenderJob`))
  (add `MoviePipelineQueueEngineSubsystem.OnRenderFinished` (`self.mrq`) (delegate `onRenderFinished`)))

(event `onRenderFinished`
  (params (Results :type "MoviePipelineOutputData Structure"))
  ; Current job is finished, iterate to the next job.
  (set `self.curCamIdx` (+ (`self.curCamIdx`) 1))
  (goto _label))

(event `self.ReceiveEndPlay`
  (params (EndPlayReason :type "EEndPlayReason Enum" :default "Destroyed"))
  ; Cleaning end the rendering process by deleting any pending jobs with mrq.
  (`self.endRenderQueue`))

(fn `calcFocalLength`
  (returns (focalLength :type "Float (double-precision)"))
  (bind _returnvalue (/ (`KismetMathLibrary.BreakVector2D` (`self.cameraSensorWidthHeight`)) (* (`KismetMathLibrary.DegTan` (/ (`self.focalLength`) 2.0)) 2.0)))
  ; Focal Length = Sensor Width / (2 x tan(fov/2))
  (`KismetSystemLibrary.PrintString` (`KismetStringLibrary.Concat_StrStr` "Focal Length:" (`KismetStringLibrary.Conv_DoubleToString` _returnvalue)) :!enabledstate Disabled)
  (return _returnvalue))

(fn `enableMediaTracks`
  (params (curCamIdx :type Integer))
  (locals (curTrack :type "MovieSceneMediaTrack Object Reference"))
  (bind _returnvalue (`MovieSceneSequenceExtensions.FindTracksByType` (`self.masterSequence`) "/Script/MediaCompositing.MovieSceneMediaTrack"))
  (for _array_element _returnvalue
    (bind _output_get (set `local.curTrack` _array_element))
    ; Does the current camera's mappings contain this media track?
    (bind _returnvalue_2 (`MovieSceneTrackExtensions.GetTrackRowDisplayName` _output_get))
    (if (`KismetArrayLibrary.Array_Contains` (`.mediaTracks_6_8899D52F40D06D06B2301E917E8C24D3` (break `/Game/Samsara/Blueprints/Camera_Blueprints/Struct_CameraConfig` (`|GetArrayItem` (`self.cameraConfig`) (`local.curCamIdx`)))) (`KismetTextLibrary.Conv_TextToString` _returnvalue_2))
      ; Get the sectinos in this track (ones that will activate / deactivate) - By default each media track only contains one section.
      (bind _returnvalue_3 (`MovieSceneTrackExtensions.GetSections` (`local.curTrack`)))
      ; Found? Mark them as active.
      ;
      ; Not found? Mark them as inactive
      (for _array_element_2 _returnvalue_3
        (`KismetSystemLibrary.PrintString` (`KismetStringLibrary.Concat_StrStr` "Active: " (`KismetSystemLibrary.GetDisplayName` _array_element_2)) true true (struct :`G` 0.66 :`B` 1.0 :`A` 1.0) 10.0 :!enabledstate Disabled)
        (`MovieSceneSection.SetIsActive` _array_element_2 true))
      (else
        (bind _returnvalue_4 (`MovieSceneTrackExtensions.GetSections` (`local.curTrack`)))
        (for _array_element_3 _returnvalue_4
          (`KismetSystemLibrary.PrintString` (`KismetStringLibrary.Concat_StrStr` "Inactive:" (`KismetSystemLibrary.GetDisplayName` _array_element_3)) true true (struct :`R` 1.0 :`G` 0.08974 :`A` 1.0) 10.0 :!enabledstate Disabled)
          (`MovieSceneSection.SetIsActive` _array_element_3 false))))))

(fn `setActiveCamera`
  (params (cameraIdx :type Integer))
  (locals (curCamera :type "CineCameraComponent Object Reference"))
  ; Activates / Deactivates a camera at camera idx (used only for sequencer to pick the right camera for rendering)
  (for (_array_element _array_index) (`self.allCameras`)
    (set `local.curCamera` _array_element)
    (if (== _array_index cameraIdx)
      (`ActorComponent.SetActive` (`local.curCamera`) true false)
      (else
        (`ActorComponent.SetActive` (`local.curCamera`) false false)))))

(fn `setupCameras`
  (locals (curCamera :type "CineCameraComponent Object Reference"))
  (bind (_x _y) (`KismetMathLibrary.BreakVector2D` (`self.cameraSensorWidthHeight`)))
  ; Creating the array of cameras
  (set `self.allCameras` (`|MakeArray` (`self.CineCamera_0`) (`self.CineCamera_1`) (`self.CineCamera_2`) (`self.CineCamera_3`) (`self.CineCamera_4`) (`self.CineCamera_5`) (`self.CineCamera_6`) (`self.CineCamera_7`) (`self.CineCamera_8`) (`self.CineCamera_9`)))
  ; Camera config is an array of CameraConfig struct. Each element is a map of camera position and videoPanel name in sequencer that the camera can see.
  (for (_array_element _array_index) (`self.cameraConfig`)
    (set `local.curCamera` (`|GetArrayItem` (`self.allCameras`) _array_index))
    ; Set camera properties
    (set `CineCameraComponent.Filmback` (make `CameraFilmbackSettings` _x _y) (`local.curCamera`))
    (`SceneComponent.K2_SetWorldTransform` (`local.curCamera`) (`KismetMathLibrary.MakeTransform` (`KismetMathLibrary.MakeVector` (.x (.location (`SplineComponent.GetTransformAtDistanceAlongSpline` (`self.splineController`) (* (`.position_9_FBC289FC4F95165443EE8EA21CD46E09` (break `/Game/Samsara/Blueprints/Camera_Blueprints/Struct_CameraConfig` _array_element)) (`self.newSplineLength`)) "World" false))) (.y (`SceneComponent.K2_GetComponentLocation` (`self.Scene`))) (.z (`SceneComponent.K2_GetComponentLocation` (`self.Scene`)))) (`KismetMathLibrary.Conv_VectorToRotator` (`KismetMathLibrary.GetReflectionVector` (`SceneComponent.GetRightVector` (`self.splineController`)) (`KismetMathLibrary.Vector_Right`)))) false false)
    (`CameraComponent.SetFieldOfView` (`local.curCamera`) 54.0)
    (set `CineCameraComponent.CurrentFocalLength` (`self.focalLength`) (`local.curCamera`))
    ; Disable Focus so exposure is same between viewport and camera
    (set `CineCameraComponent.FocusSettings` (make `CameraFocusSettings` "Disable") (`local.curCamera`))))

(fn `setupSpline`
  (locals (splinePoints :type Integer))
  (bind _returnvalue (* (`self.newSplineLength`) (`self.splineTangentLengthFactor`)))
  (bind _returnvalue_2 (* (`self.yCurveFactor`) (`self.newSplineLength`)))
  (`SplineComponent.SetLocationAtSplinePoint` (`self.splineController`) 1 (`KismetMathLibrary.MakeVector` (`self.newSplineLength`)) "Local" true)
  (set `local.splinePoints` (`SplineComponent.GetNumberOfSplinePoints` (`self.splineController`)))
  (for _index (range (+ (`local.splinePoints`) 1))
    (`SplineComponent.SetTangentsAtSplinePoint` (`self.splineController`) _index (`KismetMathLibrary.MakeVector` _returnvalue (* _returnvalue_2 -1.0)) (`KismetMathLibrary.MakeVector` _returnvalue _returnvalue_2) "World" true)))

(fn `updateOutputNames`
  (params (curJob :type "MoviePipelineExecutorJob Object Reference") (camIdx :type Integer))
  ; Job name
  (bind _output_get (set `MoviePipelineExecutorJob.JobName` (`KismetStringLibrary.Concat_StrStr` "Cam_" (`KismetStringLibrary.Conv_IntToString` camIdx)) (`local.curJob`)))
  ; Directory name
  (set `MoviePipelineOutputSetting.OutputDirectory` (make `DirectoryPath` (`KismetStringLibrary.Concat_StrStr` (`self.baseDirectory`) "\\" (`self.subDirectory`) "\\" _output_get)) (`MoviePipelineConfigBase.FindSettingByClass` (`self.renderConfig`) "/Script/MovieRenderPipelineCore.MoviePipelineOutputSetting" false false))
  ; Output filename format
  (set `MoviePipelineOutputSetting.FileNameFormat` (`KismetStringLibrary.Concat_StrStr` (`self.subDirectory`) "_" _output_get "_{frame_number}") (`MoviePipelineConfigBase.FindSettingByClass` (`self.renderConfig`) "/Script/MovieRenderPipelineCore.MoviePipelineOutputSetting" false false))
  (return))

(fn `UserConstructionScript`
  (locals (cameras :type "Array of CineCameraActor Object Reference"))
  (`self.setupSpline`)
  (`self.setupCameras`)
  ; Only used to set current camera for Sequencer
  (`self.setActiveCamera` (`KismetMathLibrary.FTrunc` (`self.curPreviewCamera`))))